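; Player character Blueprint handling movement, look, jumping, a viewport widget, background music and quitting the game.
; The Lock input toggles the mouse cursor and a Movement flag that gates walking, camera and jump input.
; Tick picks DefaultSong from BodyDiscovered, but restarts the idle audio component with a separate Music variable.
; An old line-trace interaction for InteractiveObject-tagged actors remains disconnected.
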(event `InputAction|Lock`
  (params (Key :type "Key Structure"))
  (bind _returnvalue (`GameplayStatics.GetPlayerController` 0))
  ;[1 1 1] Mouse Lock
  (:`Pressed`
    (if (`self.MouseLock`)
      (set `PlayerController.bShowMouseCursor` true _returnvalue)
      (set `self.MouseLock` false)
      (set `self.Movement` false)
      (else
        (set `PlayerController.bShowMouseCursor` false _returnvalue)
        (set `self.MouseLock` true)
        (set `self.Movement` true)))))

(event `InputAxis|Forward&Backward`
  (params (AxisValue :type "Float (single-precision)"))
  ;[1 1 1] Movement
  (if (`self.Movement`)
    (`self.AddMovementInput` (`KismetMathLibrary.GetForwardVector` (`KismetMathLibrary.MakeRotator` 0.0 0.0 (.yaw (`self.GetControlRotation`)))) AxisValue)))

(event `InputAxis|Left&Right`
  (params (AxisValue :type "Float (single-precision)"))
  ;[1 1 1] Movement
  (if (`self.Movement`)
    (`self.AddMovementInput` (`KismetMathLibrary.GetRightVector` (`KismetMathLibrary.MakeRotator` 0.0 0.0 (.yaw (`self.GetControlRotation`)))) AxisValue)))

(event `InputAction|Jump`
  (params (Key :type "Key Structure"))
  (bind _movement (`self.Movement`))
  ;[1 1 1] Camera & Jump
  (:`Pressed`
    (if _movement
      (`self.Jump`)))
  (:`Released`
    (if _movement
      (`self.StopJumping`))))

(event `InputAxis|Pitch`
  (params (AxisValue :type "Float (single-precision)"))
  ;[1 1 1] Camera & Jump
  (if (`self.Movement`)
    (`self.AddControllerPitchInput` AxisValue)))

(event `InputAction|Escape`
  (params (Key :type "Key Structure"))
  (:`Pressed`
    (`KismetSystemLibrary.QuitGame` null "Quit")))

(event `InputAxis|Yaw`
  (params (AxisValue :type "Float (single-precision)"))
  ;[1 1 1] Camera & Jump
  (if (`self.Movement`)
    (`self.AddControllerYawInput` AxisValue)))

(event `self.ReceiveBeginPlay`
  (bind _returnvalue (`|CreateWidget` "/Game/Widgets/Player_WID.Player_WID_C"))
  (`UserWidget.AddToViewport` _returnvalue 0)
  (bind _returnvalue_2 (`AddComponent|NODE_AddAudioComponent-2`))
  (set `self.Audio` _returnvalue_2))

(event `InputAction|Click`
  (params (Key :type "Key Structure"))
  ;[1 1 1] Old Click
)

(event `self.ReceiveTick`
  (params (DeltaSeconds :type "Float (single-precision)"))
  (bind _audio (`self.Audio`))
  (if (`self.BodyDiscovered`)
    (set `self.DefaultSong` "/Game/Music/investigation_3_Cue.investigation_3_Cue")
    (else
      (set `self.DefaultSong` "/Game/Music/seatheme1_Cue.seatheme1_Cue")))
  (if (not (`AudioComponent.IsPlaying` (`self.Audio`)))
    (`AudioComponent.SetSound` _audio (`self.Music`))
    (`AudioComponent.Play` _audio 0.0)))

(fn `UserConstructionScript`)