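; Player character Blueprint that handles movement, jumping, camera look and click-to-inspect, and adds the Player_WIDG widget on BeginPlay.
; Movement follows control yaw, and the Lock input toggles the mouse cursor while enabling or disabling movement, jump and look input.
; Click traces from the camera along its forward vector, printing the LookMessage of actors tagged InteractiveObject, or "No" for other hits.
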(event `InputAction|Lock`
  (params (Key :type "Key Structure"))
  (bind _returnvalue (`GameplayStatics.GetPlayerController` 0))
  ;[1 1 1] Mouse Lock
  (:`Pressed`
    (if (`self.MouseLock`)
      (set `PlayerController.bShowMouseCursor` true _returnvalue)
      (set `self.MouseLock` false)
      (set `self.Movement` false)
      (else
        (set `PlayerController.bShowMouseCursor` false _returnvalue)
        (set `self.MouseLock` true)
        (set `self.Movement` true)))))

(event `InputAxis|Forward&Backward`
  (params (AxisValue :type "Float (single-precision)"))
  ;[1 1 1] Movement
  (if (`self.Movement`)
    (`self.AddMovementInput` (`KismetMathLibrary.GetForwardVector` (`KismetMathLibrary.MakeRotator` 0.0 0.0 (.yaw (`self.GetControlRotation`)))) AxisValue)))

(event `InputAxis|Left&Right`
  (params (AxisValue :type "Float (single-precision)"))
  ;[1 1 1] Movement
  (if (`self.Movement`)
    (`self.AddMovementInput` (`KismetMathLibrary.GetRightVector` (`KismetMathLibrary.MakeRotator` 0.0 0.0 (.yaw (`self.GetControlRotation`)))) AxisValue)))

(event `InputAction|Jump`
  (params (Key :type "Key Structure"))
  (bind _movement (`self.Movement`))
  ;[1 1 1] Camera & Jump
  (:`Pressed`
    (if _movement
      (`self.Jump`)))
  (:`Released`
    (if _movement
      (`self.StopJumping`))))

(event `InputAxis|Pitch`
  (params (AxisValue :type "Float (single-precision)"))
  ;[1 1 1] Camera & Jump
  (if (`self.Movement`)
    (`self.AddControllerPitchInput` AxisValue)))

(event `InputAxis|Yaw`
  (params (AxisValue :type "Float (single-precision)"))
  ;[1 1 1] Camera & Jump
  (if (`self.Movement`)
    (`self.AddControllerYawInput` AxisValue)))

(event `self.ReceiveBeginPlay`
  (bind _returnvalue (`|CreateWidget` "/Game/Widgets/Player_WIDG.Player_WIDG_C"))
  (`UserWidget.AddToViewport` _returnvalue 0))

(event `InputAction|Click`
  (params (Key :type "Key Structure"))
  (bind _returnvalue (`GameplayStatics.GetPlayerCameraManager` 0))
  (bind _returnvalue_2 (`self.K2_GetActorLocation` _returnvalue))
  (:`Pressed`
    (bind (_outhit _returnvalue_3) (`KismetSystemLibrary.LineTraceSingle` _returnvalue_2 (+ (* (`self.GetActorForwardVector` _returnvalue) 5000.0) _returnvalue_2) "TraceTypeQuery1"))
    (if _returnvalue_3
      (bind (_bblockinghit _binitialoverlap _time _distance _location _impactpoint _normal _impactnormal _physmat _hitactor) (`GameplayStatics.BreakHitResult` _outhit))
      (if (`self.ActorHasTag` _hitactor "InteractiveObject")
        (bind _output (message `/Game/Blueprints/InterfaceBP.Look` _hitactor))
        (`KismetSystemLibrary.PrintString` _output)
        (else
          (`KismetSystemLibrary.PrintString` "No"))))))

(fn `UserConstructionScript`)