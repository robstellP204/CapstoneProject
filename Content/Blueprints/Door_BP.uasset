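; Door actor that answers Look, Talk and Use interactions with dialogue and warps the player elsewhere when used.
; Look and Talk only return their dialogue variables.
; Use teleports the player character to WarpLocation, stops the audio on Player_BP, and sets its Music to one of two songs based on BodyDiscovered.
; It then returns the Use dialogue; playback of the new song is not started here.
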(fn `Look`
  (returns (Output :type String))
  (return (`self.LookDialogue`)))

(fn `Talk`
  (returns (Dialogue :type String))
  (return (`self.TalkDialogue`)))

(fn `Use`
  (returns (String :type String))
  (bind _returnvalue (`GameplayStatics.GetPlayerCharacter` 0))
  (`self.K2_SetActorLocation` _returnvalue (`self.WarpLocation`) false true)
  (bind _asplayer_bp (cast `/Game/Blueprints/Player_BP` _returnvalue))
  (`AudioComponent.Stop` (`/Game/Blueprints/Player_BP.Audio` _asplayer_bp))
  (if (`/Game/Blueprints/Player_BP.BodyDiscovered` _asplayer_bp)
    (set `/Game/Blueprints/Player_BP.Music` (`self.SongValue2`) _asplayer_bp)
    (else
      (set `/Game/Blueprints/Player_BP.Music` (`self.SongValue1`) _asplayer_bp)))
  (return (`self.UseDialogue`)))

(fn `UserConstructionScript`)