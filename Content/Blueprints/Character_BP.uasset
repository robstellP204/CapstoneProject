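; Character_BP is an NPC for a dialogue-driven story with a body discovery, turning to face the player every tick.
; BeginPlay caches DialogueSpreadsheet rows matching its NPCID, and Talk looks up the line for the current ConversationID and LineID.
; Ending key conversations with Marie, Frank or Jacob sets trigger flags on Player_BP.
; GetConvo polls those flags each tick, advancing every NPC's conversation stage in sequence through LineManager.
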(event `self.ReceiveBeginPlay`
  ;[1 1 1] Data Table Array & Player Set-Up
  (bind _outrownames (`DataTableFunctionLibrary.GetDataTableRowNames` "/Game/Blueprints/DialogueSpreadsheet.DialogueSpreadsheet"))
  (for _array_element _outrownames
    (bind _returnvalue (`|GetDataTableRow` "/Game/Blueprints/DialogueSpreadsheet.DialogueSpreadsheet" _array_element)
      (:`then`
        (if (== (`.NPC_ID_2_B81F1C64452FA676747870BFD1ED26C6` (break `/Game/Blueprints/DialogueStruct` _returnvalue)) (`self.NPC_ID`))
          (`KismetArrayLibrary.Array_Add` (`self.Dialogue`) (`KismetStringLibrary.Conv_NameToString` _array_element))
          (bind _asplayer_bp (cast `/Game/Blueprints/Player_BP` (`GameplayStatics.GetPlayerCharacter` 0)))
          (set `self.Player` _asplayer_bp))))))

(event `self.ReceiveTick`
  (params (DeltaSeconds :type "Float (single-precision)"))
  (bind (_returnvalue_roll _returnvalue_pitch _returnvalue_yaw) (`KismetMathLibrary.BreakRotator` (`KismetMathLibrary.FindLookAtRotation` (`self.K2_GetActorLocation`) (`self.K2_GetActorLocation` (`GameplayStatics.GetPlayerCharacter` 0)))))
  ;[1 1 1] Rotator & Conversation Call
  (`self.K2_SetActorRotation` (`KismetMathLibrary.MakeRotator` 0.0 0.0 _returnvalue_yaw))
  (`self.GetConvo`))

(fn `GetConvo`
  (bind _player (`self.Player`))
  (bind _asplayer_bp (cast `/Game/Blueprints/Player_BP` (`GameplayStatics.GetPlayerCharacter` 0)))
  (if (and (`/Game/Blueprints/Player_BP.BodyDiscovered` _asplayer_bp) (`KismetStringLibrary.EqualEqual_StrStr` (`self.LineManager`) "Line1"))
    (set `self.Conversation_ID` 2)
    (set `self.Line_ID` 1)
    (set `self.LineManager` "Line2"))
  (if (`/Game/Blueprints/Player_BP.MarieTrigger` (`self.Player`))
    (if (`KismetStringLibrary.EqualEqual_StrStr` (`self.LineManager`) "Line2")
      (set `self.Conversation_ID` 3)
      (set `self.Line_ID` 1)
      (set `self.LineManager` "Line3")))
  (if (and (`/Game/Blueprints/Player_BP.FrankTrigger` (`self.Player`)) (`KismetStringLibrary.EqualEqual_StrStr` (`self.LineManager`) "Line3"))
    (set `self.Conversation_ID` 4)
    (set `self.Line_ID` 1)
    (set `self.LineManager` "Line4"))
  (if (and (`/Game/Blueprints/Player_BP.JacobTrigger` (`self.Player`)) (`KismetStringLibrary.EqualEqual_StrStr` (`self.LineManager`) "Line4"))
    (set `self.Conversation_ID` 5)
    (set `self.Line_ID` 1)
    (set `self.LineManager` "Line5"))
  (if (and (and (`/Game/Blueprints/Player_BP.MarieTrigger2` _player) (`/Game/Blueprints/Player_BP.FrankTrigger2` _player)) (`KismetStringLibrary.EqualEqual_StrStr` (`self.LineManager`) "Line5"))
    (set `self.Conversation_ID` 6)
    (set `self.Line_ID` 1)
    (set `self.LineManager` "Line6")))

(fn `Look`
  (returns (Output :type String))
  (return ""))

(fn `Talk`
  (returns (Dialogue :type String))
  (locals (ReturnedLines :type "Array of String"))
  ;[1 1 1] Talk Function
  (for _array_element (`self.Dialogue`)
    (bind _returnvalue (`|GetDataTableRow` "/Game/Blueprints/DialogueSpreadsheet.DialogueSpreadsheet" (`KismetStringLibrary.Conv_StringToName` _array_element))
      (:`then`
        (bind (_npc_id _conversation_id _line_id _dialogue) (break `/Game/Blueprints/DialogueStruct` _returnvalue))
        (if (and (== _conversation_id (`self.Conversation_ID`)) (== _line_id (`self.Line_ID`)))
          (`KismetArrayLibrary.Array_Add` (`local.ReturnedLines`) _dialogue)
          ;[1 1 1] Events in Dialogue
          (if (and (`KismetStringLibrary.EqualEqual_StrStr` (`|GetArrayItem` (`local.ReturnedLines`)) "END") (and (== (`self.Conversation_ID`) 2) (`KismetStringLibrary.EqualEqual_StrStr` (`self.Name`) "Marie")))
            (set `/Game/Blueprints/Player_BP.MarieTrigger` true (`self.Player`)))
          (if (and (`KismetStringLibrary.EqualEqual_StrStr` (`|GetArrayItem` (`local.ReturnedLines`)) "END") (and (== (`self.Conversation_ID`) 3) (`KismetStringLibrary.EqualEqual_StrStr` (`self.Name`) "Frank")))
            (set `/Game/Blueprints/Player_BP.FrankTrigger` true (`self.Player`)))
          (if (and (`KismetStringLibrary.EqualEqual_StrStr` (`|GetArrayItem` (`local.ReturnedLines`)) "END") (and (== (`self.Conversation_ID`) 4) (`KismetStringLibrary.EqualEqual_StrStr` (`self.Name`) "Jacob")))
            (set `/Game/Blueprints/Player_BP.JacobTrigger` true (`self.Player`)))
          (if (and (`KismetStringLibrary.EqualEqual_StrStr` (`|GetArrayItem` (`local.ReturnedLines`)) "END") (and (== (`self.Conversation_ID`) 5) (`KismetStringLibrary.EqualEqual_StrStr` (`self.Name`) "Marie")))
            (set `/Game/Blueprints/Player_BP.MarieTrigger2` true (`self.Player`)))
          (if (and (`KismetStringLibrary.EqualEqual_StrStr` (`|GetArrayItem` (`local.ReturnedLines`)) "END") (and (== (`self.Conversation_ID`) 5) (`KismetStringLibrary.EqualEqual_StrStr` (`self.Name`) "Frank")))
            (set `/Game/Blueprints/Player_BP.FrankTrigger2` true (`self.Player`)))))))
  (if (== (`KismetArrayLibrary.Array_Length` (`local.ReturnedLines`)) 1)
    (return (`|GetArrayItem` (`local.ReturnedLines`)))
    (else
      (set `self.Line_ID` 0))))

(fn `Use`
  (returns (String :type String))
  (return ""))

(fn `UserConstructionScript`)