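; DeadMan_BP is the murdered passenger's corpse, an interactable in a mystery investigation that answers Look, Talk and Use with descriptive text.
; Each Tick it sets its yaw to face the player character, billboard-style.
; Look also sets BodyDiscovered on Player_BP, recording that the player has found the body, while Talk and Use only return flavour text.
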(event `self.ReceiveTick`
  (params (DeltaSeconds :type "Float (single-precision)"))
  (bind (_returnvalue_roll _returnvalue_pitch _returnvalue_yaw) (`KismetMathLibrary.BreakRotator` (`KismetMathLibrary.FindLookAtRotation` (`self.K2_GetActorLocation`) (`self.K2_GetActorLocation` (`GameplayStatics.GetPlayerCharacter` 0)))))
  (`self.K2_SetActorRotation` (`KismetMathLibrary.MakeRotator` 0.0 0.0 _returnvalue_yaw)))

(fn `Look`
  (returns (Output :type String))
  (bind _asplayer_bp (cast `/Game/Blueprints/Player_BP` (`GameplayStatics.GetPlayerCharacter` 0)))
  (set `/Game/Blueprints/Player_BP.BodyDiscovered` true _asplayer_bp)
  (return "The corpse has stab wounds and is covered in lipstick. You should ask the other passengers about this..."))

(fn `Talk`
  (returns (Dialogue :type String))
  (return "There's no response. It's just a corpse."))

(fn `Use`
  (returns (String :type String))
  (return "You can't do anything with the corpse. Besides, you should leave this for the cops..."))

(fn `UserConstructionScript`)